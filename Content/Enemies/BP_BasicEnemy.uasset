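; BP_BasicEnemy is a simple enemy that loses health when hit by projectiles and is destroyed when it runs out.
; The construction script sets starting health and a fixed per-hit damage, so the enemy itself determines damage taken.
; A hit on the Model component casts the other actor to BP_Projectile, subtracts damage and destroys the enemy at exactly zero health.
; Debug strings print the remaining health, death and non-projectile hits.
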(event OnComponentHit(Model)
  (params (HitComponent :type Primitive%20Component%20Object%20Reference) (OtherActor :type Actor%20Object%20Reference) (OtherComp :type Primitive%20Component%20Object%20Reference) (NormalImpulse :type Vector :default "0, 0, 0") (Hit :type Hit%20Result%20Structure%20%28by%20ref%29))
  (Utilities|Casting|CastToBP_Projectile OtherActor
    (:then
      (bind _output_get (Variables|Default|SetHealth (- (Variables|Default|GetHealth) (Variables|Default|GetDamge))))
      (Development|PrintString (Utilities|String|ToString(Integer) _output_get))
      (if (== (Variables|Default|GetHealth) 0)
        (Actor|DestroyActor)
        (Development|PrintString "bye :3")))
    (:CastFailed
      (Development|PrintString "nuh uh"))))

(fn ConstructionScript
  (Variables|Default|SetHealth 50)
  (Variables|Default|SetDamge 10))