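; BP_Enemy is an enemy character that takes damage from projectiles and can chase a seen pawn.
; Capsule hits from BP_Projectile subtract its own Damage, set in the construction script, from Health, destroying it when Health equals exactly zero.
; PawnSensing flags the player as seen, but only ranged enemies then follow using AI MoveTo.
; A helper function sets maximum walk speed, and debug prints report health and death.
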(event OnComponentHit(CapsuleComponent)
  (params (HitComponent :type Primitive%20Component%20Object%20Reference) (OtherActor :type Actor%20Object%20Reference) (OtherComp :type Primitive%20Component%20Object%20Reference) (NormalImpulse :type Vector :default "0, 0, 0") (Hit :type Hit%20Result%20Structure%20%28by%20ref%29))
  (Utilities|Casting|CastToBP_Projectile OtherActor)
  (bind _output_get (Variables|Default|SetHealth (- (Variables|Default|GetHealth) (Variables|Default|GetDamage))))
  (Development|PrintString (Utilities|String|ToString(Integer) _output_get))
  (if (== (Variables|Default|GetHealth) 0)
    (Actor|DestroyActor)
    (Development|PrintString "bye :3")))

(event OnSeePawn(PawnSensing)
  (params (Pawn :type Pawn%20Object%20Reference))
  (Variables|Default|SetIsPlayerSeen? true)
  (if (Variables|Default|GetisRanged?)
    (CallFunction|FollowPlayer)))

(event Custom|FollowPlayer
  (if (Variables|Default|GetIsPlayerSeen?)
    (AI|AIMoveTo self "0, 0, 0" (stale OnSeePawn(PawnSensing) Pawn) 5.0 false)))

(fn ConstructionScript
  (Variables|Default|SetDamage 5))

(fn UpdateWalkSpeed
  (params (New%20Walk%20Speed :type Float%20%28double-precision%29))
  (Variables|/Script/Engine.CharacterMovementComponent|SetMaxWalkSpeed (Variables|Character|GetCharacterMovement) New%20Walk%20Speed))